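; BP_DoubleLeverDoor is a castle door wrapper that opens a BP_DoubleDoor_Interior held in its child actor component.
; Tick watches for IsOpen differing from its cached value and, only when it turns true, sets IsOpen on the child door.
; Closing is not forwarded, and nothing in this file sets IsOpen.
; BeginPlay stores identical open and closed positions, prints the child's location and re-applies it unchanged.
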(event `self.ReceiveBeginPlay`
  (bind _returnvalue (`self.K2_GetActorLocation`))
  (bind _childactor (`ChildActorComponent.ChildActor` (`self.ChildActor`)))
  (bind _returnvalue_2 (`self.K2_GetActorLocation` _childactor))
  (set `self.OpenPosition` _returnvalue)
  (set `self.ClosedPosition` _returnvalue)
  (`KismetSystemLibrary.PrintString` (`KismetStringLibrary.Conv_VectorToString` _returnvalue_2))
  (`self.K2_SetActorLocation` _childactor _returnvalue_2 false false))

(event `self.ReceiveTick`
  (params (DeltaSeconds :type "Float (single-precision)"))
  (bind _isopen (`self.IsOpen`))
  (if (!= (`self.cacheOpen`) (`self.IsOpen`))
    (if _isopen
      (bind _asbp_double_door_interior (cast `/Game/OneStarPrison/Blueprints/Castle/BP_DoubleDoor_Interior` (`ChildActorComponent.ChildActor` (`self.ChildActor`))))
      (set `DoubleDoorCastle.IsOpen` true _asbp_double_door_interior)
      (set `self.cacheOpen` _isopen))))

(fn `UserConstructionScript`)