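; BP_FullMazeDoor is a castle maze door actor that wraps a BP_RotateMazeDoubleDoor child actor.
; On Tick it compares IsOpen to a cached value, passes any change to the child door and plays that door's OpenSound at its own location.
; The same sound plays for both opening and closing.
; BeginPlay sets both the open and closed positions to the actor's own location, so movement is left to the child.
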(event `self.ReceiveBeginPlay`
  (bind _returnvalue (`self.K2_GetActorLocation`))
  (set `self.OpenPosition` _returnvalue)
  (set `self.ClosedPosition` _returnvalue))

(event `self.ReceiveTick`
  (params (DeltaSeconds :type "Float (single-precision)"))
  (if (!= (`self.cacheOpen`) (`self.IsOpen`))
    (bind _asbp_rotate_maze_double_door (cast `/Game/OneStarPrison/Blueprints/Castle/BP_RotateMazeDoubleDoor` (`ChildActorComponent.ChildActor` (`self.MazeDoors`))))
    (bind _output_get (set `DoubleDoorCastle.IsOpen` (`self.IsOpen`) _asbp_rotate_maze_double_door))
    (`GameplayStatics.PlaySoundAtLocation` (`DoubleDoorCastle.OpenSound` _asbp_rotate_maze_double_door) (`self.K2_GetActorLocation`) (struct) 1.0 1.0 0.0 null null null null)
    (set `self.cacheOpen` _output_get)))

(fn `UserConstructionScript`)