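; BP_Curtain is a castle curtain actor that animates opening and closing by scaling its skeletal mesh.
; Each Tick, it eases the mesh's world scale toward full size when IsOpen is true, or toward a narrow X scale when false.
; The lerp starts from the current scale with an alpha of delta time times OpenCloseSpeed, giving a decelerating motion.
; Nothing in this graph changes IsOpen.
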(event `self.ReceiveTick`
  (params (DeltaSeconds :type "Float (single-precision)"))
  (bind _skeletalmesh (`self.SkeletalMesh`))
  (bind _skeletalmesh_2 (`self.SkeletalMesh`))
  (bind _returnvalue (* DeltaSeconds (`self.OpenCloseSpeed`)))
  (if (`self.IsOpen`)
    (`SceneComponent.SetWorldScale3D` _skeletalmesh_2 (`KismetMathLibrary.VLerp` (`SceneComponent.K2_GetComponentScale` _skeletalmesh_2) (1.0 1.0 1.0) _returnvalue))
    (else
      (`SceneComponent.SetWorldScale3D` _skeletalmesh (`KismetMathLibrary.VLerp` (`SceneComponent.K2_GetComponentScale` _skeletalmesh) (0.1 1.0 1.0) _returnvalue)))))

(fn `UserConstructionScript`)