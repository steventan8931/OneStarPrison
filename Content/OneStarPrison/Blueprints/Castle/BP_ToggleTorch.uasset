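; BP_ToggleTorch is a castle torch that can be shown lit or unlit through an IsOn flag.
; On BeginPlay a timeline drives the point light's intensity, scaled by a large multiplier.
; Every Tick it reads IsOn to show or hide the Lights component with its children and to unpause or pause the two Firepit components.
; The flag is only read here, not set.
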(event `self.ReceiveBeginPlay`
  (bind (_direction _intensity) (`Timeline|Timeline_0`)
    (:`Update`
      (`LightComponent.SetIntensity` (`self.PointLight`) (* _intensity 100000.0)))))

(event `self.ReceiveTick`
  (params (DeltaSeconds :type "Float (single-precision)"))
  (bind _firepit (`self.firepit`))
  (bind _firepit1 (`self.firepit1`))
  (if (`self.IsOn`)
    (`SceneComponent.SetVisibility` (`self.Lights`) true true)
    (`AudioComponent.SetPaused` _firepit false)
    (`AudioComponent.SetPaused` _firepit1 false)
    (else
      (`SceneComponent.SetVisibility` (`self.Lights`) false true)
      (`AudioComponent.SetPaused` _firepit true)
      (`AudioComponent.SetPaused` _firepit1 true))))

(fn `UserConstructionScript`)