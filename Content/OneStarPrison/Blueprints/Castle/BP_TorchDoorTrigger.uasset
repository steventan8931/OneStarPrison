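; BP_TorchDoorTrigger is a castle trigger volume that opens linked doors when the required number of players stand inside, optionally needing a carried key.
; Begin and end overlaps track the player count, light or douse one linked torch per player, and cache any key holder.
; Tick compares the count, destroys the held key when one is required, and opens the doors, which either latch open or close when the count stops matching.
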(event `self.ReceiveActorBeginOverlap`
  (params (OtherActor :type "Actor Object Reference"))
  (if (not (`self.DoorOpen`))
    (bind _asbp_player_character (cast `/Game/OneStarPrison/Blueprints/BP_PlayerCharacter` OtherActor))
    (bind _pickedupitem (`PlayerCharacter.PickedUpItem` _asbp_player_character))
    (if (!= _pickedupitem null)
      (bind _asbp_pickupable_key (cast `/Game/OneStarPrison/Blueprints/BP_PickupableKey` _pickedupitem)
        (:`then`
          (set `self.HasKey` true)
          (set `self.CachePlayer` _asbp_player_character)
          (set `self.CacheKey` _asbp_pickupable_key))
        (:`CastFailed`
          _)))
    (set `self.PlayerCount` (+ (`self.PlayerCount`) 1))
    (for _array_element (`self.ToggleTorch`)
      (if (not (`/Game/OneStarPrison/Blueprints/Castle/BP_ToggleTorch.IsOn` _array_element))
        (set `/Game/OneStarPrison/Blueprints/Castle/BP_ToggleTorch.IsOn` true _array_element)
        (break)))))

(event `self.ReceiveActorEndOverlap`
  (params (OtherActor :type "Actor Object Reference"))
  (if (not (`self.DoorOpen`))
    (bind _asbp_player_character (cast `/Game/OneStarPrison/Blueprints/BP_PlayerCharacter` OtherActor))
    (bind _pickedupitem (`PlayerCharacter.PickedUpItem` _asbp_player_character))
    (if (!= _pickedupitem null)
      (cast `/Game/OneStarPrison/Blueprints/BP_PickupableKey` _pickedupitem
        (:`then`
          (set `self.HasKey` false)
          (set `self.CachePlayer` null)
          (set `self.CacheKey` null))
        (:`CastFailed`
          _)))
    (set `self.PlayerCount` (+ (`self.PlayerCount`) -1))
    (for _array_element (`self.ToggleTorch`)
      (if (`/Game/OneStarPrison/Blueprints/Castle/BP_ToggleTorch.IsOn` _array_element)
        (set `/Game/OneStarPrison/Blueprints/Castle/BP_ToggleTorch.IsOn` false _array_element)
        (break)))))

(event `self.ReceiveTick`
  (params (DeltaSeconds :type "Float (single-precision)"))
  (bind _cacheplayer (`self.CachePlayer`))
  (bind _pickedupitem (`PlayerCharacter.PickedUpItem` _cacheplayer))
  (if (== (`self.PlayerCount`) (`self.PlayerCountNeeded`))
    (if (`self.NeedsKey`)
      (if (`self.HasKey`)
        (if (!= _cacheplayer null)
          (if (!= _pickedupitem null)
            (bind _asbp_pickupable_key (cast `/Game/OneStarPrison/Blueprints/BP_PickupableKey` _pickedupitem))
            (bind _output_get (set `self.CacheKey` _asbp_pickupable_key))
            (`self.K2_DestroyActor` _output_get)
            (set `PlayerCharacter.PickedUpItem` null _cacheplayer)
            (for _array_element (`self.Doors`) :!label _label
              (set `Door.IsOpen` true _array_element))
            (if (`self.StaysOpen`)
              (set `self.DoorOpen` true)))))
      (else
        (goto _label)))
    (elif (not (`self.StaysOpen`))
      (for _array_element_2 (`self.Doors`)
        (set `Door.IsOpen` false _array_element_2)))))

(fn `UserConstructionScript`)