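; BP_CastleCurtain is a castle curtain barrier that closes while a player character is inside its trigger box and reopens when they leave.
; Box1 overlaps toggle an invisible Collision blocker, set IsOpen on the BP_Curtain child actor and play a curtain sound.
; It starts open on BeginPlay.
; PlayersInside is set to 1 or 0 rather than counted, so any player exiting reopens it.
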(event `self.Box1.OnComponentBeginOverlap`
  (params (OverlappedComponent :type "PrimitiveComponent Object Reference") (OtherActor :type "Actor Object Reference") (OtherComp :type "PrimitiveComponent Object Reference") (OtherBodyIndex :type Integer) (bFromSweep :type Boolean) (SweepResult :type "HitResult Structure (by ref)"))
  (bind _collision (`self.Collision`))
  (bind _childactor (`ChildActorComponent.ChildActor` (`self.ChildActor`)))
  (bind _asbp_player_character (cast `/Game/OneStarPrison/Blueprints/BP_PlayerCharacter` OtherActor))
  (set `self.FirstPlayer` _asbp_player_character)
  (set `self.PlayersInside` 1)
  (`SceneComponent.SetVisibility` _collision false false)
  (`PrimitiveComponent.SetCollisionEnabled` _collision "QueryAndPhysics")
  (bind _asbp_curtain (cast `/Game/OneStarPrison/Blueprints/Castle/BP_Curtain` _childactor))
  (set `/Game/OneStarPrison/Blueprints/Castle/BP_Curtain.IsOpen` false _asbp_curtain)
  (`GameplayStatics.PlaySoundAtLocation` "/Game/OneStarPrison/Sounds/Castle/Curtain_Sound.Curtain_Sound" (`self.K2_GetActorLocation` _childactor) (struct) 1.0 1.0 0.0 null null null null))

(event `self.Box1.OnComponentEndOverlap`
  (params (OverlappedComponent :type "PrimitiveComponent Object Reference") (OtherActor :type "Actor Object Reference") (OtherComp :type "PrimitiveComponent Object Reference") (OtherBodyIndex :type Integer))
  (bind _collision (`self.Collision`))
  (bind _childactor (`ChildActorComponent.ChildActor` (`self.ChildActor`)))
  (cast `/Game/OneStarPrison/Blueprints/BP_PlayerCharacter` OtherActor)
  (set `self.PlayersInside` 0)
  (`SceneComponent.SetVisibility` _collision false false)
  (`PrimitiveComponent.SetCollisionEnabled` _collision "NoCollision")
  (bind _asbp_curtain (cast `/Game/OneStarPrison/Blueprints/Castle/BP_Curtain` _childactor))
  (set `/Game/OneStarPrison/Blueprints/Castle/BP_Curtain.IsOpen` true _asbp_curtain)
  (`GameplayStatics.PlaySoundAtLocation` "/Game/OneStarPrison/Sounds/Castle/Curtain_Sound.Curtain_Sound" (`self.K2_GetActorLocation` _childactor) (struct) 1.0 1.0 0.0 null null null null))

(event `self.ReceiveBeginPlay`
  (bind _collision (`self.Collision`))
  (`SceneComponent.SetVisibility` _collision false false)
  (`PrimitiveComponent.SetCollisionEnabled` _collision "NoCollision")
  (bind _asbp_curtain (cast `/Game/OneStarPrison/Blueprints/Castle/BP_Curtain` (`ChildActorComponent.ChildActor` (`self.ChildActor`))))
  (set `/Game/OneStarPrison/Blueprints/Castle/BP_Curtain.IsOpen` true _asbp_curtain))

(fn `UserConstructionScript`)