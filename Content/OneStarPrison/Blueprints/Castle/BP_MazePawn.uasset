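; BP_MazePawn is a castle maze pawn that eases its camera into place when possessed.
; First possession stores the camera's own transform as the target, then every possession snaps the camera to CurrentCameraTransform.
; Tick lerps it back by delta time until nearly equal, then sets CanMove, which unpossessing clears.
; Movement is unimplemented: CanMove only triggers a debug print.
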(event `self.ReceiveBeginPlay`)

(event `self.ReceivePossessed`
  (params (NewController :type "Controller Object Reference"))
  (if (`self.FirstFrame`)
    (set `self.EndCameraTransform` (`SceneComponent.K2_GetComponentToWorld` (`self.Cam`)))
    (set `self.FirstFrame` false))
  (`SceneComponent.K2_SetWorldTransform` (`self.Cam`) (`self.CurrentCameraTransform`) false false))

(event `Key|W`
  (params (Key :type "Key Structure")))

(event `self.ReceiveUnpossessed`
  (params (OldController :type "Controller Object Reference"))
  (set `self.CanMove` false))

(event `self.ReceiveTick`
  (params (DeltaSeconds :type "Float (single-precision)"))
  (bind _endcameratransform (`self.EndCameraTransform`))
  (bind _returnvalue (`SceneComponent.K2_GetComponentToWorld` (`self.Cam`)))
  (if (`self.CanMove`)
    (`KismetSystemLibrary.PrintString` "Hello")
    (else
      (`SceneComponent.K2_SetWorldTransform` (`self.Cam`) (`KismetMathLibrary.TLerp` _returnvalue _endcameratransform (`GameplayStatics.GetWorldDeltaSeconds`)) false false)
      (if (`KismetMathLibrary.NearlyEqual_TransformTransform` _returnvalue _endcameratransform 20.0 20.0 5.0)
        (set `self.CanMove` true)))))

(fn `UserConstructionScript`)