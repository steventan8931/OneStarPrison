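; BP_BarrelKey is a key actor that can fly as a projectile and is tied to the castle trap room.
; Hitting anything other than the player switches it to physics simulation, stops projectile movement, clears its in-air state and plays a sound.
; It caches any trap room trigger it overlaps, and Tick destroys the key whenever that trigger is not in its triggered state.
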(event `self.ReceiveBeginPlay`)

(event `self.ReceiveActorBeginOverlap`
  (params (OtherActor :type "Actor Object Reference"))
  (bind _asbp_trap_room_trigger (cast `/Game/OneStarPrison/Blueprints/Castle/BP_TrapRoomTrigger` OtherActor))
  (set `self.TrapTrigger` _asbp_trap_room_trigger))

(event `self.ReceiveTick`
  (params (DeltaSeconds :type "Float (single-precision)"))
  (bind _traptrigger (`self.TrapTrigger`))
  (if (!= _traptrigger null)
    (if (not (`TrapRoomTrigger.Triggered` _traptrigger))
      (`self.K2_DestroyActor`))))

(event `self.ReceiveHit`
  (params (MyComp :type "PrimitiveComponent Object Reference") (Other :type "Actor Object Reference") (OtherComp :type "PrimitiveComponent Object Reference") (bSelfMoved :type Boolean) (HitLocation :type "Vector Structure") (HitNormal :type "Vector Structure") (NormalImpulse :type "Vector Structure") (Hit :type "HitResult Structure (by ref)"))
  (cast `/Game/OneStarPrison/Blueprints/BP_PlayerCharacter` Other
    (:`CastFailed`
      (`PrimitiveComponent.SetSimulatePhysics` (`self.Mesh`) true)
      (`ActorComponent.Deactivate` (`self.ProjectileMovement`))
      (set `self.IsInAir` false)
      (`GameplayStatics.PlaySoundAtLocation` "/Game/OneStarPrison/Sounds/keyhit.keyhit" (`self.K2_GetActorLocation`) (struct) 1.0 1.0 0.0 null null null null))))

(fn `UserConstructionScript`)