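; BP_PossessTriggertest is a trigger actor that hands player control from BP_PlayerCharacter to a BP_MazePawn when the character overlaps it.
; On overlap it zeroes the character's velocity, then casts its Pawn variable to BP_MazePawn.
; It passes the character and its camera boom's world transform to the maze pawn before player controller 0 possesses that pawn.
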(event `self.ReceiveActorBeginOverlap`
  (params (OtherActor :type "Actor Object Reference"))
  (bind _pawn (`self.Pawn`))
  (bind _asbp_player_character (cast `/Game/OneStarPrison/Blueprints/BP_PlayerCharacter` OtherActor))
  (set `MovementComponent.Velocity` (0.0 0.0 0.0) (`Character.CharacterMovement` _asbp_player_character))
  (bind _asbp_maze_pawn (cast `/Game/OneStarPrison/Blueprints/Castle/BP_MazePawn` _pawn))
  (set `MazePawn.CurrentPlayer` _asbp_player_character _asbp_maze_pawn)
  (set `MazePawn.CurrentCameraTransform` (`SceneComponent.K2_GetComponentToWorld` (`PlayerCharacter.CameraBoom` _asbp_player_character)) _asbp_maze_pawn)
  (`Controller.Possess` (`GameplayStatics.GetPlayerController` 0) _pawn))

(fn `UserConstructionScript`)