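; Castle set-dressing bookshelf actor that randomizes its rows of books at runtime.
; On BeginPlay it gathers the Shelf's direct child static mesh components into BookRows, then loops over them to assign one of three book row meshes at random.
; A Delay sits inside that loop, so the swap likely reaches only the last row.
; The debug-printed random number is rolled separately from the one choosing the mesh.
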(event `self.ReceiveBeginPlay`
  (bind _returnvalue (`KismetMathLibrary.RandomIntegerInRange` 0 2))
  (for _array_element (`SceneComponent.GetChildrenComponents` (`self.Shelf`) false)
    (bind _asstatic_mesh_component (cast `StaticMeshComponent` _array_element))
    (`KismetArrayLibrary.Array_Add` (`self.BookRows`) _asstatic_mesh_component))
  (for _array_element_2 (`self.BookRows`)
    (`KismetSystemLibrary.Delay` 0.1)
    (`KismetSystemLibrary.PrintString` (`KismetStringLibrary.Conv_IntToString` _returnvalue))
    (switch `int` _returnvalue
      (:`0`
        (`StaticMeshComponent.SetStaticMesh` _array_element_2 "/Game/Props/Castle_props/BookRow_V1.BookRow_V1"))
      (:`1`
        (`StaticMeshComponent.SetStaticMesh` _array_element_2 "/Game/Props/Castle_props/BookRow_V2.BookRow_V2"))
      (:`2`
        (`StaticMeshComponent.SetStaticMesh` _array_element_2 "/Game/Props/Castle_props/BookRow_V3.BookRow_V3")))))

(fn `UserConstructionScript`)