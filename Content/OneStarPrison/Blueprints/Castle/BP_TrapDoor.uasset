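; BP_TrapDoor is a castle trap door actor that gives audio feedback when its open state changes.
; Tick compares IsOpen with a cached copy and plays OpenSound at the actor's location on any change, opening or closing.
; The graph only reads IsOpen and never sets it.
; A branch that would toggle mesh collision from IsOpen is disconnected and never runs.
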(event `self.ReceiveTick`
  (params (DeltaSeconds :type "Float (single-precision)"))
  (bind _isopen (`self.IsOpen`))
  (if (!= (`self.cacheOpen`) _isopen)
    (`GameplayStatics.PlaySoundAtLocation` (`self.OpenSound`) (`self.K2_GetActorLocation`) (struct) 0.5 1.0 0.0 null null null null)
    (set `self.cacheOpen` _isopen)))

(fn `UserConstructionScript`)