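; BP_DoubleLeverDoor_Alt is a castle door Blueprint that relays its open state to a referenced DoubleLeverDoor.
; Tick compares IsOpen with CacheOpen and, when it turns true and the reference is set, sets that door's IsOpen and updates the cache.
; Closing is never forwarded or cached.
; BeginPlay stores the actor's location as both open and closed positions, but the graph never moves the actor.
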(event `self.ReceiveBeginPlay`
  (bind _returnvalue (`self.K2_GetActorLocation`))
  (set `self.OpenPosition` _returnvalue)
  (set `self.ClosedPosition` _returnvalue))

(event `self.ReceiveTick`
  (params (DeltaSeconds :type "Float (single-precision)"))
  (bind _isopen (`self.IsOpen`))
  (bind _doubleleverdoor (`self.DoubleLeverDoor`))
  (if (!= (`self.cacheOpen`) (`self.IsOpen`))
    (if _isopen
      (if (!= _doubleleverdoor null)
        (set `DoubleDoorCastle.IsOpen` true _doubleleverdoor)
        (set `self.cacheOpen` _isopen)))))

(fn `UserConstructionScript`)