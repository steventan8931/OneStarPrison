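; Test maze-watcher pawn for the castle that takes over the view with a camera transition while possessed.
; On possession it saves its camera's transform as the target, then snaps the camera to the CurrentCamera transform.
; Tick eases the camera back toward that target by lerping from its present transform with delta seconds as alpha.
; Space bar makes player controller 0 possess CurrentPlayer, handing control back.
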(event `self.ReceiveBeginPlay`)

(event `self.ReceivePossessed`
  (params (NewController :type "Controller Object Reference"))
  (set `self.EndCamera` (`SceneComponent.K2_GetComponentToWorld` (`self.Camera`)))
  (`SceneComponent.K2_SetWorldTransform` (`self.Camera`) (`self.CurrentCamera`) false false))

(event `Key|SpaceBar`
  (params (Key :type "Key Structure"))
  (:`Pressed`
    (`Controller.Possess` (`GameplayStatics.GetPlayerController` 0) (`self.CurrentPlayer`))))

(event `self.ReceiveTick`
  (params (DeltaSeconds :type "Float (single-precision)"))
  (`SceneComponent.K2_SetWorldTransform` (`self.Camera`) (`KismetMathLibrary.TLerp` (`SceneComponent.K2_GetComponentToWorld` (`self.Camera`)) (`self.EndCamera`) (`GameplayStatics.GetWorldDeltaSeconds`)) false false))

(fn `UserConstructionScript`)