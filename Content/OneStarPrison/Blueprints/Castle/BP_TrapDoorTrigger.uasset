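; A castle trigger volume that opens linked trap doors while two player characters stand inside it.
; Overlap begin and end events track the player count and light or extinguish one linked torch per player, showing occupancy.
; Tick sets the doors open when the count is exactly two, then uses an accumulated timer to hold them open for a configurable time before closing them.
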(event `self.ReceiveActorBeginOverlap`
  (params (OtherActor :type "Actor Object Reference"))
  (cast `/Game/OneStarPrison/Blueprints/BP_PlayerCharacter` OtherActor)
  (set `self.PlayerCount` (+ (`self.PlayerCount`) 1))
  (for _array_element (`self.ToggleTorch`)
    (if (not (`/Game/OneStarPrison/Blueprints/Castle/BP_ToggleTorch.IsOn` _array_element))
      (set `/Game/OneStarPrison/Blueprints/Castle/BP_ToggleTorch.IsOn` true _array_element)
      (break))))

(event `self.ReceiveActorEndOverlap`
  (params (OtherActor :type "Actor Object Reference"))
  (cast `/Game/OneStarPrison/Blueprints/BP_PlayerCharacter` OtherActor)
  (set `self.PlayerCount` (+ (`self.PlayerCount`) -1))
  (for _array_element (`self.ToggleTorch`)
    (if (`/Game/OneStarPrison/Blueprints/Castle/BP_ToggleTorch.IsOn` _array_element)
      (set `/Game/OneStarPrison/Blueprints/Castle/BP_ToggleTorch.IsOn` false _array_element)
      (break))))

(event `self.ReceiveTick`
  (params (DeltaSeconds :type "Float (single-precision)"))
  (if (== (`self.PlayerCount`) 2)
    (for _array_element (`self.TrapDoors`)
      (set `Door.IsOpen` true _array_element)
      (set `self.RecentlyOpen` true))
    (elif (`self.RecentlyOpen`)
      (bind _output_get (set `self.OpenTimer` (+ DeltaSeconds (`self.OpenTimer`))))
      (if (>= _output_get (`self.TimeToStayOpen`))
        (set `self.RecentlyOpen` false)
        (set `self.OpenTimer` 0.0))
      (else
        (for _array_element_2 (`self.TrapDoors`)
          (set `Door.IsOpen` false _array_element_2))))))

(fn `UserConstructionScript`)