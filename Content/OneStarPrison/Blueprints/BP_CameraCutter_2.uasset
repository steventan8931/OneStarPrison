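; BP_CameraCutter_2 is a trigger actor that briefly cuts a player's camera to itself when a BP_PlayerCharacter overlaps it.
; If that character has a valid local viewing player controller, the view target blends to this actor.
; After a short delay, the character's ResetCameraToPlayer restores the view.
; Disconnected leftover nodes for moving and deactivating components never run.
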(event `self.ReceiveActorBeginOverlap`
  (params (OtherActor :type "Actor Object Reference"))
  (bind _asbp_player_character (cast `/Game/OneStarPrison/Blueprints/BP_PlayerCharacter` OtherActor))
  (bind _returnvalue (`Pawn.GetLocalViewingPlayerController` _asbp_player_character))
  (if (`KismetSystemLibrary.IsValid` _returnvalue)
    (`PlayerController.SetViewTargetWithBlend` _returnvalue self 1.0 "VTBlend_Linear" 1.0 false)
    (`KismetSystemLibrary.Delay` 2.0)
    (`/Game/OneStarPrison/Blueprints/BP_PlayerCharacter.ResetCameraToPlayer` _asbp_player_character)))

(fn `UserConstructionScript`)