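; Player character for a networked game, handling settings and character-select menus, ready state and a choice of themed character models.
; Client and server events manage story or free-play selection widgets and ready status.
; UpdateCharacterModel swaps meshes through client and server events, saving the choice to player state and game instance, with delayed model updates on BeginPlay.
; Tick reports noise when moving uncrouched, and F12 restarts the level.
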(event `ClientSettings`
  (bind _returnvalue (`|CreateWidget` "/Game/OneStarPrison/UI/WBP_Settings.WBP_Settings_C" (`self.GetLocalViewingPlayerController`)))
  (`UserWidget.AddToPlayerScreen` _returnvalue 0)
  (set `self.SettingsWidget` _returnvalue)
  (set `PlayerController.bShowMouseCursor` true (`GameplayStatics.GetPlayerController` 0)))

(event `ClientRemoveSettings`
  (bind _settingswidget (`self.SettingsWidget`))
  (if (!= _settingswidget null)
    (`Widget.RemoveFromParent` _settingswidget)
    (set `PlayerController.bShowMouseCursor` false (`GameplayStatics.GetPlayerController` 0))
    (set `self.SettingsWidget` null)))

(event `ServerCharacterSelect`
  (params (`Is Free Play` :type Boolean))
  (`/Engine/EditorBlueprintResources/ActorMacros.Switch Has Authority`
    (:`Authority`
      (`self.ClientChracterSelect` `Is Free Play`))))

(event `ClientChracterSelect`
  (params (IsFreePlay :type Boolean))
  (bind _returnvalue (`self.GetLocalViewingPlayerController`))
  (if IsFreePlay
    (bind _returnvalue_2 (`|CreateWidget` "/Game/OneStarPrison/UI/WBP_CharacterSelect_Freeplay.WBP_CharacterSelect_Freeplay_C" _returnvalue))
    (`UserWidget.AddToPlayerScreen` _returnvalue_2 0)
    (set `self.FreePlaySelectWidget` _returnvalue_2)
    (else
      (bind _returnvalue_3 (`|CreateWidget` "/Game/OneStarPrison/UI/WBP_CharacterSelect_Story.WBP_CharacterSelect_Story_C" _returnvalue (`self.ModelOptionM`) (`self.ModelOptionF`)))
      (`UserWidget.AddToPlayerScreen` _returnvalue_3 0)
      (set `self.CharacterSelectWidget` _returnvalue_3)))
  (set `PlayerController.bShowMouseCursor` true (`GameplayStatics.GetPlayerController` 0)))

(event `ServerRemoveCharacterSelect`
  (params (IsFreePlay :type Boolean))
  (`self.ClientRemoveCharacterSelect` IsFreePlay))

(event `Key|F12`
  (params (Key :type "Key Structure"))
  (:`Pressed`
    (bind _asbp_level_game_mode (cast `/Game/OneStarPrison/Blueprints/BP_LevelGameMode` (`GameplayStatics.GetGameMode`)))
    (`/Game/OneStarPrison/Blueprints/BP_LevelGameMode.Restart Level` _asbp_level_game_mode)))

(event `ClientRemoveCharacterSelect`
  (params (IsFreePlay :type Boolean))
  (bind _characterselectwidget (`self.CharacterSelectWidget`))
  (bind _freeplayselectwidget (`self.FreePlaySelectWidget`))
  (if IsFreePlay
    (if (!= _freeplayselectwidget null)
      (`Widget.RemoveFromParent` _freeplayselectwidget)
      (set `PlayerController.bShowMouseCursor` false (`GameplayStatics.GetPlayerController` 0) :!label _label))
    (elif (!= _characterselectwidget null)
      (`Widget.RemoveFromParent` _characterselectwidget)
      (goto _label))))

(event `Key|One`
  (params (Key :type "Key Structure"))
  (:`Pressed`
    (if (!= (`self.SettingsWidget`) null) :!label _label_2
      (`self.ClientRemoveSettings`)
      (else
        (`self.ClientSettings`)))))

(event `Key|Escape`
  (params (Key :type "Key Structure"))
  (:`Pressed`
    (goto _label_2)))

(event `ClientSetReady`
  (params (IsReady :type Boolean))
  (`self.ServerSetReady` IsReady))

(event `self.ReceiveBeginPlay`
  (`|ExecutionSequence`
    (:`then_0`
      (`/Engine/EditorBlueprintResources/ActorMacros.Switch Has Authority`
        (:`Authority`
          (`KismetSystemLibrary.Delay` 1.0)
          (if (`Controller.IsLocalPlayerController` (`GameplayStatics.GetPlayerController` 0))
            (bind _asbp_player_state (cast `/Game/OneStarPrison/Saves/BP_PlayerState` (`GameplayStatics.GetPlayerState` 0)))
            (`/Game/OneStarPrison/Saves/BP_PlayerState.Update Model` _asbp_player_state)
            (set `self.IsHost` true)))))
    (:`then_1`
      (`/Engine/EditorBlueprintResources/ActorMacros.Switch Has Authority`
        (:`Remote`
          (`KismetSystemLibrary.Delay` 2.0)
          (bind _asbp_advanced_game_instance (cast `/Game/OneStarPrison/Network/BP_AdvancedGameInstance` (`GameplayStatics.GetGameInstance`)))
          (`/Game/OneStarPrison/Network/BP_AdvancedGameInstance.Update Model` _asbp_advanced_game_instance)
          (set `self.IsHost` false))))))

(event `ServerSetReady`
  (params (IsReady :type Boolean))
  (set `self.IsReady` IsReady))

(event `UpdateModelClient`
  (params (NewMesh :type "SkeletalMesh Object Reference"))
  (`/Engine/EditorBlueprintResources/ActorMacros.Switch Has Authority`
    (:`Remote`
      (`SkinnedMeshComponent.SetSkinnedAssetAndUpdate` (`self.Mesh`) NewMesh true)
      (bind _asbp_player_state (cast `/Game/OneStarPrison/Saves/BP_PlayerState` (`self.PlayerState`) :!label _label_3))
      (set `/Game/OneStarPrison/Saves/BP_PlayerState.Saved Model` (`self.ModelType`) _asbp_player_state))))

(event `Key|One`
  (params (Key :type "Key Structure")))

(event `ChangeModelServer`
  (params (NewMesh :type "SkeletalMesh Object Reference"))
  (`/Engine/EditorBlueprintResources/ActorMacros.Switch Has Authority`
    (:`Authority`
      (`|ExecutionSequence`
        (:`then_0`
          (`SkinnedMeshComponent.SetSkinnedAssetAndUpdate` (`self.Mesh`) NewMesh true)
          (bind _asbp_player_state (cast `/Game/OneStarPrison/Saves/BP_PlayerState` (`self.PlayerState`)))
          (set `/Game/OneStarPrison/Saves/BP_PlayerState.Saved Model` (`self.ModelType`) _asbp_player_state)
          (bind _asbp_advanced_game_instance (cast `/Game/OneStarPrison/Network/BP_AdvancedGameInstance` (`GameplayStatics.GetGameInstance`)))
          (set `/Game/OneStarPrison/Network/BP_AdvancedGameInstance.Saved Model Type` (`self.ModelType`) _asbp_advanced_game_instance))
        (:`then_1`
          (goto _label_3))))))

(event `Key|Two`
  (params (Key :type "Key Structure")))

(event `self.ReceiveTick`
  (params (DeltaSeconds :type "Float (single-precision)"))
  (if (== (`MovementComponent.Velocity` (`self.CharacterMovement`)) (0.0 0.0 0.0))
    (set `self.IsPushing` false)
    (elif (not (`self.IsCrouching`))
      (`AISense_Hearing.ReportNoiseEvent` (`self.K2_GetActorLocation`) 1.0 self))))

(event `Key|Three`
  (params (Key :type "Key Structure")))

(fn `Update Character Model`
  (params (`Model Type` :type "/Game/OneStarPrison/Enumerations/ECharacterModel Enum" :default "NewEnumerator0"))
  (bind _output_get (set `self.ModelType` `Model Type`))
  (bind _asbp_player_state (cast `/Game/OneStarPrison/Saves/BP_PlayerState` (`GameplayStatics.GetPlayerState` 0)))
  (bind _output_get_2 (set `/Game/OneStarPrison/Saves/BP_PlayerState.Saved Model` _output_get _asbp_player_state))
  (switch `/Game/OneStarPrison/Enumerations/ECharacterModel` _output_get_2
    (:`NewEnumerator0`
      (`self.UpdateModelClient` "/Game/OneStarPrison/Assets/Character/Character_Male.Character_Male")
      (`self.ChangeModelServer` "/Game/OneStarPrison/Assets/Character/Character_Male.Character_Male"))
    (:`NewEnumerator1`
      (`self.UpdateModelClient` "/Game/OneStarPrison/Assets/Female_Character/Female_Model.Female_Model")
      (`self.ChangeModelServer` "/Game/OneStarPrison/Assets/Female_Character/Female_Model.Female_Model"))
    (:`NewEnumerator2`
      (`self.UpdateModelClient` "/Game/OneStarPrison/Assets/Character/Caveman_Model/CaveMan.CaveMan")
      (`self.ChangeModelServer` "/Game/OneStarPrison/Assets/Character/Caveman_Model/CaveMan.CaveMan"))
    (:`NewEnumerator5`
      (`self.UpdateModelClient` "/Game/OneStarPrison/Assets/Character/Female_Caveman_model/The_CaveWoman.The_CaveWoman")
      (`self.ChangeModelServer` "/Game/OneStarPrison/Assets/Character/Female_Caveman_model/The_CaveWoman.The_CaveWoman"))
    (:`NewEnumerator3`
      (`self.UpdateModelClient` "/Game/OneStarPrison/Assets/Character/Pirate/Pirate.Pirate")
      (`self.ChangeModelServer` "/Game/OneStarPrison/Assets/Character/Pirate/Pirate.Pirate"))
    (:`NewEnumerator4`
      (`self.UpdateModelClient` "/Game/OneStarPrison/Assets/Character/FemalePirate/Pirate_Lady.Pirate_Lady")
      (`self.ChangeModelServer` "/Game/OneStarPrison/Assets/Character/FemalePirate/Pirate_Lady.Pirate_Lady"))))

(fn `UserConstructionScript`)