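; Level select trigger that moves the session to another map when a BP_PlayerCharacter overlaps it.
; ChangeLevel appends MapName to a servertravel console command and executes it on player controller 0.
; CheckIsReady sets LobbyReady from the IsReady flags in Players, but nothing in this file calls it or gates the travel on it.
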(event `self.ReceiveTick`
  (params (DeltaSeconds :type "Float (single-precision)")))

(event `self.ReceiveActorBeginOverlap`
  (params (OtherActor :type "Actor Object Reference"))
  (cast `/Game/OneStarPrison/Blueprints/BP_PlayerCharacter` OtherActor)
  (`self.Change Level`))

(event `Change Level`
  (`KismetSystemLibrary.ExecuteConsoleCommand` (`KismetStringLibrary.Concat_StrStr` "servertravel " (`self.MapName`)) (`GameplayStatics.GetPlayerController` 0)))

(fn `CheckIsReady`
  (for _array_element (`self.Players`)
    (if (`/Game/OneStarPrison/Blueprints/BP_PlayerCharacter.IsReady` _array_element)
      (set `self.LobbyReady` true)
      (else
        (set `self.LobbyReady` false)
        (break)))))

(fn `UserConstructionScript`)