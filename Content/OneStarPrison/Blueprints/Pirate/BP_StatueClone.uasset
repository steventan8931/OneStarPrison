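; BP_StatueClone is a pirate-area statue that mirrors the appearance of another statue given by StatueReference.
; On Tick, while FirstFrame is set, it waits for a non-empty reference, copies that statue's top, middle and bottom row values, then calls UpdateVisibility.
; It also takes the source's animal mesh and clears FirstFrame, so the copy happens once and later changes to the source are not followed.
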(event `self.ReceiveTick`
  (params (DeltaSeconds :type "Float (single-precision)"))
  (bind _statuereference (`self.StatueReference`))
  (if (`self.FirstFrame`)
    (if (!= _statuereference null)
      (set `self.TopRow` (`Statue.TopRow` _statuereference))
      (set `self.MidRow` (`Statue.MidRow` _statuereference))
      (set `self.BotRow` (`Statue.BotRow` _statuereference))
      (`self.UpdateVisibility`)
      (`StaticMeshComponent.SetStaticMesh` (`self.AnimalMesh`) (`StaticMeshComponent.StaticMesh` (`Statue.AnimalMesh` _statuereference)))
      (set `self.FirstFrame` false))))

(event `self.ReceiveBeginPlay`)

(fn `UserConstructionScript`)