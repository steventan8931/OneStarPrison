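; BP_GhostLight is a light actor that deals SunShine damage wherever its beam lands, apparently aimed at ghost enemies.
; Each tick it traces along its Arrow's forward vector and moves a Sphere to the hit point, scaled by hit distance.
; Radial damage is applied there, with a radius that widens with distance like a cone.
; An unconnected point-damage branch casting to Enemy_Ghost never runs.
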(event `self.ReceiveTick`
  (params (DeltaSeconds :type "Float (single-precision)"))
  (bind _sphere (`self.Sphere`))
  (bind _returnvalue (`self.K2_GetActorLocation` self))
  (bind _outhit (`KismetSystemLibrary.LineTraceSingle` _returnvalue (+ _returnvalue (* (`SceneComponent.GetForwardVector` (`self.Arrow`)) 50000.0)) "TraceTypeQuery1"))
  (bind (_bblockinghit _binitialoverlap _time _distance _location) (`GameplayStatics.BreakHitResult` _outhit))
  (set `self.Location` _location)
  (`SceneComponent.K2_SetWorldLocation` _sphere _location false false)
  (`SceneComponent.SetRelativeScale3D` _sphere (`KismetMathLibrary.Conv_DoubleToVector` (* _distance 0.006)))
  (`GameplayStatics.ApplyRadialDamage` :`BaseDamage` 10.0 :`Origin` _location :`DamageRadius` (* _distance (`KismetMathLibrary.DegSin` 12.0)) :`DamageTypeClass` "/Game/AI/CPP/SunShine.SunShine_C" :`DamageCauser` null :`InstigatedByController` null))

(event `self.ReceiveActorBeginOverlap`
  (params (OtherActor :type "Actor Object Reference")))

(fn `UserConstructionScript`)