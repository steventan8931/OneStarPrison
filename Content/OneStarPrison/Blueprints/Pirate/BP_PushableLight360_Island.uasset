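; Pushable light Blueprint for the pirate island that projects a damaging spot of light where its Arrow points.
; Each tick, a camera-channel trace from the Arrow moves a Sphere to the hit point and scales it with distance, like a 15-degree beam cone.
; It applies SunShine radial damage there, using that distance-based radius as both reach and damage amount.
; The Cone overlap, NPC blackboard logic and debug-sphere variant are unconnected leftovers.
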(event `self.ReceiveTick`
  (params (DeltaSeconds :type "Float (single-precision)"))
  (bind _sphere (`self.Sphere`))
  (bind _returnvalue (`SceneComponent.K2_GetComponentLocation` (`self.Arrow`)))
  (bind _outhit (`KismetSystemLibrary.LineTraceSingle` :`Start` _returnvalue :`End` (+ _returnvalue (* (`SceneComponent.GetForwardVector` (`self.Arrow`)) 50000.0)) :`TraceChannel` "TraceTypeQuery2" :`DrawTime` 0.0))
  (bind (_bblockinghit _binitialoverlap _time _distance _location) (`GameplayStatics.BreakHitResult` _outhit))
  (bind _returnvalue_2 (+ _location (0.0 0.0 1.0)))
  (set `self.Location` _returnvalue_2)
  (`SceneComponent.K2_SetWorldLocation` _sphere _returnvalue_2 false false)
  (bind _returnvalue_3 (* _distance (`KismetMathLibrary.DegSin` 15.0)))
  (`SceneComponent.SetRelativeScale3D` _sphere (`KismetMathLibrary.Conv_DoubleToVector` (/ _returnvalue_3 50.0)))
  (`GameplayStatics.ApplyRadialDamage` :`BaseDamage` _returnvalue_3 :`Origin` _returnvalue_2 :`DamageRadius` _returnvalue_3 :`DamageTypeClass` "/Game/AI/CPP/SunShine.SunShine_C" :`DamageCauser` null :`InstigatedByController` null :`bDoFullDamage` true :`DamagePreventionChannel` "ECC_WorldStatic"))

(event `self.Cone.OnComponentBeginOverlap`
  (params (OverlappedComponent :type "PrimitiveComponent Object Reference") (OtherActor :type "Actor Object Reference") (OtherComp :type "PrimitiveComponent Object Reference") (OtherBodyIndex :type Integer) (bFromSweep :type Boolean) (SweepResult :type "HitResult Structure (by ref)")))

(fn `UserConstructionScript`)