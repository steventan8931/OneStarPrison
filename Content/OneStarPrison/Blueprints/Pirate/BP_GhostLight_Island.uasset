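; Pirate-level ghost light island actor that hosts a child light actor and keeps its rotation in step with a lighthouse light.
; On BeginPlay, if flashing is enabled, it passes the flashing flag and delay to its child BP_PushableLight360.
; Every Tick it reads the world rotation of the mesh on the referenced Lighthouse's child light and applies it as the relative rotation of its own child's root.
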(event `self.ReceiveBeginPlay`
  (bind _isflashing (`self.IsFlashing`))
  (if _isflashing
    (bind _asbp_pushable_light_360 (cast `/Game/OneStarPrison/Blueprints/Pirate/BP_PushableLight360` (`ChildActorComponent.ChildActor` (`self.ChildActor`))))
    (set `/Game/OneStarPrison/Blueprints/Pirate/BP_PushableLight360.IsFlashing` _isflashing _asbp_pushable_light_360)
    (set `/Game/OneStarPrison/Blueprints/Pirate/BP_PushableLight360.FlashDelay` (`self.FlashDelay`) _asbp_pushable_light_360)))

(event `self.ReceiveTick`
  (params (DeltaSeconds :type "Float (single-precision)"))
  (bind _childactor (`ChildActorComponent.ChildActor` (`self.ChildActor`)))
  (bind _childactor_2 (`ChildActorComponent.ChildActor` (`/Game/OneStarPrison/Blueprints/Pirate/BP_GhostLight_Lighthouse.ChildActor` (`self.Lighthouse`))))
  (if (`KismetSystemLibrary.IsValid` _childactor_2)
    (bind _asbp_pushable_light_360_lighthouse (cast `/Game/OneStarPrison/Blueprints/Pirate/BP_PushableLight360_Lighthouse` _childactor_2))
    (if (`KismetSystemLibrary.IsValid` _childactor)
      (bind _mesh (`Pushable.Mesh` _asbp_pushable_light_360_lighthouse))
      (if (`KismetSystemLibrary.IsValid` _mesh)
        (`SceneComponent.K2_SetRelativeRotation` (`Actor.RootComponent` _childactor) (`SceneComponent.K2_GetComponentRotation` _mesh) false false)))))

(fn `UserConstructionScript`)