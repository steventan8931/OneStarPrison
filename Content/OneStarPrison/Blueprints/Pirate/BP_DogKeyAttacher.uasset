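; BP_DogKeyAttacher is a trigger actor that makes an enemy dog pick up a referenced key.
; On actor overlap, it casts to Enemy_Dog and, if the key is set, attaches it to the dog's Bone_025 socket.
; It then plays a pickup sound, nudges the key mesh with a local offset and sets IsTaken so the pickup happens only once.
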(event `self.ReceiveActorBeginOverlap`
  (params (OtherActor :type "Actor Object Reference"))
  (bind _key (`self.Key`))
  (if (not (`self.IsTaken`))
    (bind _asenemy_dog (cast `/Game/AI/CPP/Enemy_Dog` OtherActor))
    (if (!= _key null)
      (`self.K2_AttachToActor` _key _asenemy_dog "Bone_025" "SnapToTarget" "KeepWorld" "KeepWorld" false)
      (`GameplayStatics.PlaySoundAtLocation` "/Game/OneStarPrison/Sounds/keypickup.keypickup" (`self.K2_GetActorLocation`) (struct) 1.0 1.0 0.0 null null null null)
      (`SceneComponent.K2_AddLocalOffset` (`Pickupable.Mesh` _key) (60.0 0.0 0.0) false false)
      (set `self.IsTaken` true))))

(fn `UserConstructionScript`)