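; BP_Dinghy is a pirate dinghy actor that bobs and rocks in place.
; Each Tick adds small cosine-driven local offsets in Z and rotations in roll, pitch and yaw to its static mesh, using time since creation.
; The vertical motion is phase-shifted from the rotation.
; Increments are applied per frame without delta-time scaling, so the motion's amplitude depends on frame rate.
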(event `self.ReceiveTick`
  (params (DeltaSeconds :type "Float (single-precision)"))
  (bind _returnvalue (`KismetMathLibrary.Cos` (+ (`self.GetGameTimeSinceCreation`) 0.0)))
  (bind _returnvalue_2 (* _returnvalue -0.05))
  (`SceneComponent.K2_AddLocalOffset` (`self.StaticMesh`) (`KismetMathLibrary.MakeVector` 0.0 0.0 (* (`KismetMathLibrary.Cos` (+ (`self.GetGameTimeSinceCreation`) 2.0)) 0.5)) false false)
  (`SceneComponent.K2_AddLocalRotation` (`self.StaticMesh`) (`KismetMathLibrary.MakeRotator` (* _returnvalue 0.05) _returnvalue_2 _returnvalue_2) false false))

(fn `UserConstructionScript`)