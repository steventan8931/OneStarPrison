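; Pirate-themed sign actor that reflects a statue manager's completion progress by toggling three numbered components.
; Every Tick it polls StatueManager.TimesCompleted and switches on the count.
; Counts one to three cumulatively hide components 1 through 3 via fall-through wiring.
; At zero it shows 1 and 3 but hides 2, which this graph never makes visible.
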(event `self.ReceiveTick`
  (params (DeltaSeconds :type "Float (single-precision)"))
  (bind _statuemanager (`self.StatueManager`))
  (if (!= _statuemanager null)
    (switch `int` (`StatueManager.TimesCompleted` _statuemanager)
      (:`0`
        (`SceneComponent.SetVisibility` (`self.1`) true false)
        (`SceneComponent.SetVisibility` (`self.2`) false false)
        (`SceneComponent.SetVisibility` (`self.3`) true false))
      (:`1`
        (`SceneComponent.SetVisibility` (`self.1`) false false :!label _label))
      (:`2`
        (`SceneComponent.SetVisibility` (`self.2`) false false :!label _label_2)
        (goto _label))
      (:`3`
        (`SceneComponent.SetVisibility` (`self.3`) false false)
        (goto _label_2)))))

(fn `UserConstructionScript`)