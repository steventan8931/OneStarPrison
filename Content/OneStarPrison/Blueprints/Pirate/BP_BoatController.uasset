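; BP_BoatController is the pirate boat's rowing control that swaps its own mesh for rowing meshes on the player using it.
; Each Tick, while the overlapping player is interacting, it hides its Mesh and shows that player's left or right row mesh based on IsRowingRight.
; Otherwise it shows its Mesh again and hides both row meshes on any still-overlapping player.
; The graph only toggles visibility; it does not set the overlap or rowing state.
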(event `self.ReceiveTick`
  (params (DeltaSeconds :type "Float (single-precision)"))
  (bind _overlappingplayer (`self.OverlappingPlayer`))
  (bind _mesh (`self.Mesh`))
  (if (!= _overlappingplayer null)
    (if (`PlayerCharacter.IsInteracting` _overlappingplayer)
      (`SceneComponent.SetVisibility` _mesh false false)
      (bind _asbp_player_character (cast `/Game/OneStarPrison/Blueprints/BP_PlayerCharacter` _overlappingplayer))
      (if (`self.IsRowingRight`)
        (bind _rowleftmesh (`/Game/OneStarPrison/Blueprints/BP_PlayerCharacter.RowLeftMesh` _asbp_player_character))
        (`SceneComponent.SetVisibility` _rowleftmesh false false)
        (bind _rowrightmesh (`/Game/OneStarPrison/Blueprints/BP_PlayerCharacter.RowRightMesh` _asbp_player_character))
        (`SceneComponent.SetVisibility` _rowrightmesh true false)
        (else
          (`SceneComponent.SetVisibility` _rowleftmesh true false)
          (`SceneComponent.SetVisibility` _rowrightmesh false false)))
      (else
        (`SceneComponent.SetVisibility` _mesh true false :!label _label)
        (bind _asbp_player_character_2 (cast `/Game/OneStarPrison/Blueprints/BP_PlayerCharacter` _overlappingplayer))
        (`SceneComponent.SetVisibility` (`/Game/OneStarPrison/Blueprints/BP_PlayerCharacter.RowLeftMesh` _asbp_player_character_2) false false)
        (`SceneComponent.SetVisibility` (`/Game/OneStarPrison/Blueprints/BP_PlayerCharacter.RowRightMesh` _asbp_player_character_2) false false)))
    (else
      (goto _label))))

(fn `UserConstructionScript`)