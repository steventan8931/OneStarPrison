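; BP_LoadLevelTrigger is a lobby trigger that moves the session to another map once two players are inside and ready.
; Overlap events track player characters and their count, starting character selection on entry and removing selection and ready state on exit.
; With exactly two players, Tick checks that all are ready, then runs a servertravel console command built from MapName through player controller 0.
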(event `self.ReceiveActorBeginOverlap`
  (params (OtherActor :type "Actor Object Reference"))
  (bind _asbp_player_character (cast `/Game/OneStarPrison/Blueprints/BP_PlayerCharacter` OtherActor))
  (set `self.PlayerCount` (+ (`self.PlayerCount`) 1))
  (`/Game/OneStarPrison/Blueprints/BP_PlayerCharacter.ServerCharacterSelect` _asbp_player_character)
  (`KismetArrayLibrary.Array_Add` (`self.Players`) _asbp_player_character))

(event `self.ReceiveActorEndOverlap`
  (params (OtherActor :type "Actor Object Reference"))
  (bind _asbp_player_character (cast `/Game/OneStarPrison/Blueprints/BP_PlayerCharacter` OtherActor))
  (set `self.PlayerCount` (+ (`self.PlayerCount`) -1))
  (`/Game/OneStarPrison/Blueprints/BP_PlayerCharacter.ServerRemoveCharacterSelect` _asbp_player_character)
  (set `/Game/OneStarPrison/Blueprints/BP_PlayerCharacter.IsReady` false _asbp_player_character)
  (`KismetArrayLibrary.Array_RemoveItem` (`self.Players`) _asbp_player_character))

(event `self.ReceiveTick`
  (params (DeltaSeconds :type "Float (single-precision)"))
  (if (== (`self.PlayerCount`) 2)
    (`self.CheckIsReady`)
    (if (`self.LobbyReady`)
      (`self.Change Level`)
      (`KismetSystemLibrary.PrintString` "New Level"))))

(event `Change Level`
  (`KismetSystemLibrary.ExecuteConsoleCommand` (`KismetStringLibrary.Concat_StrStr` "servertravel " (`self.MapName`)) (`GameplayStatics.GetPlayerController` 0)))

(fn `CheckIsReady`
  (for _array_element (`self.Players`)
    (if (`/Game/OneStarPrison/Blueprints/BP_PlayerCharacter.IsReady` _array_element)
      (set `self.LobbyReady` true)
      (else
        (set `self.LobbyReady` false)
        (break)))))

(fn `UserConstructionScript`)