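; Game mode for One Star Prison levels that handles restarting, returning to the menu and saving era progression.
; ReturnToMainMenu and RestartLevel issue servertravel console commands to the level select lobby or the current level, then remove all widgets.
; UnlockLevel loads or creates a BP_LevelCompletionSave in slot "1", marks the given era completed and unlocks the next in the Caveman, Medieval, Pirate chain, then saves.
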(event `Return To Main Menu`
  (`KismetSystemLibrary.ExecuteConsoleCommand` (`KismetStringLibrary.Concat_StrStr` "servertravel " "LevelSelectLobbyGame") (`GameplayStatics.GetPlayerController` 0))
  (`WidgetLayoutLibrary.RemoveAllWidgets`))

(event `Restart Level`
  (bind _returnvalue (`GameplayStatics.GetCurrentLevelName` true))
  (`KismetSystemLibrary.ExecuteConsoleCommand` (`KismetStringLibrary.Concat_StrStr` "servertravel " _returnvalue) (`GameplayStatics.GetPlayerController` 0))
  (`WidgetLayoutLibrary.RemoveAllWidgets`))

(fn `Unlock Level`
  (params (EraToUnlock :type "/Game/OneStarPrison/Enumerations/ELevelEras Enum" :default "NewEnumerator0"))
  (bind _returnvalue (`GameplayStatics.LoadGameFromSlot` "1"))
  (if (!= _returnvalue null)
    (bind _asbp_level_completion_save (cast `/Game/OneStarPrison/Saves/BP_LevelCompletionSave` _returnvalue))
    (switch `/Game/OneStarPrison/Enumerations/ELevelEras` EraToUnlock
      (:`NewEnumerator0`
        (setmembers `/Game/OneStarPrison/Saves/F_LevelStatus` :`StructRef` (`/Game/OneStarPrison/Saves/BP_LevelCompletionSave.Caveman` _asbp_level_completion_save) :`Completed` true)
        (bind _medieval (`/Game/OneStarPrison/Saves/BP_LevelCompletionSave.Medieval` _asbp_level_completion_save))
        (setmembers `/Game/OneStarPrison/Saves/F_LevelStatus` :`StructRef` _medieval :`Unlocked` true))
      (:`NewEnumerator1`
        (setmembers `/Game/OneStarPrison/Saves/F_LevelStatus` :`StructRef` _medieval :`Completed` true)
        (bind _pirate (`/Game/OneStarPrison/Saves/BP_LevelCompletionSave.Pirate` _asbp_level_completion_save))
        (setmembers `/Game/OneStarPrison/Saves/F_LevelStatus` :`StructRef` _pirate :`Unlocked` true))
      (:`NewEnumerator2`
        (setmembers `/Game/OneStarPrison/Saves/F_LevelStatus` :`StructRef` _pirate :`Completed` true)))
    (`GameplayStatics.SaveGameToSlot` _asbp_level_completion_save "1")
    (else
      (bind _returnvalue_2 (`GameplayStatics.CreateSaveGameObject` "/Game/OneStarPrison/Saves/BP_LevelCompletionSave.BP_LevelCompletionSave_C"))
      (switch `/Game/OneStarPrison/Enumerations/ELevelEras` EraToUnlock
        (:`NewEnumerator0`
          (setmembers `/Game/OneStarPrison/Saves/F_LevelStatus` :`StructRef` (`/Game/OneStarPrison/Saves/BP_LevelCompletionSave.Caveman` _returnvalue_2) :`Completed` true)
          (bind _medieval_2 (`/Game/OneStarPrison/Saves/BP_LevelCompletionSave.Medieval` _returnvalue_2))
          (setmembers `/Game/OneStarPrison/Saves/F_LevelStatus` :`StructRef` _medieval_2 :`Unlocked` true))
        (:`NewEnumerator1`
          (setmembers `/Game/OneStarPrison/Saves/F_LevelStatus` :`StructRef` _medieval_2 :`Completed` true)
          (bind _pirate_2 (`/Game/OneStarPrison/Saves/BP_LevelCompletionSave.Pirate` _returnvalue_2))
          (setmembers `/Game/OneStarPrison/Saves/F_LevelStatus` :`StructRef` _pirate_2 :`Unlocked` true))
        (:`NewEnumerator2`
          (setmembers `/Game/OneStarPrison/Saves/F_LevelStatus` :`StructRef` _pirate_2 :`Completed` true)))
      (`GameplayStatics.SaveGameToSlot` _returnvalue_2 "1"))))

(fn `UserConstructionScript`)