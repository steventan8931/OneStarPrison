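; Trigger box that ends the game when both players stand inside it.
; Overlap begin and end events count BP_PlayerCharacter actors within the box.
; Tick checks for a count of two and, only once, shows the WBP_GameEnd widget.
; It then shows player 0's mouse cursor and switches that controller to UI-only input focused on the widget.
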(event `self.ReceiveActorBeginOverlap`
  (params (OtherActor :type "Actor Object Reference"))
  (cast `/Game/OneStarPrison/Blueprints/BP_PlayerCharacter` OtherActor)
  (set `self.PlayerCount` (+ (`self.PlayerCount`) 1)))

(event `self.ReceiveActorEndOverlap`
  (params (OtherActor :type "Actor Object Reference"))
  (cast `/Game/OneStarPrison/Blueprints/BP_PlayerCharacter` OtherActor)
  (set `self.PlayerCount` (+ (`self.PlayerCount`) -1)))

(event `self.ReceiveTick`
  (params (DeltaSeconds :type "Float (single-precision)"))
  (bind _returnvalue (`GameplayStatics.GetPlayerController` 0))
  (if (and (== (`self.PlayerCount`) 2) (== (`self.UI_Poped`) false))
    (bind _returnvalue_2 (`|CreateWidget` "/Game/OneStarPrison/UI/WBP_GameEnd.WBP_GameEnd_C"))
    (`UserWidget.AddToViewport` _returnvalue_2 0)
    (set `self.UI_Poped` true)
    (set `PlayerController.bShowMouseCursor` true _returnvalue)
    (`WidgetBlueprintLibrary.SetInputMode_UIOnlyEx` _returnvalue _returnvalue_2)))

(fn `UserConstructionScript`)