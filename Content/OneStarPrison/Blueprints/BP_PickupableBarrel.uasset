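; Pickupable barrel that a player carries in hand and that drops into physics when it hits something.
; While a player is set and OnDisplay is true, Tick stops its movement, snaps it to the palm socket as a trigger and applies a one-time grip offset.
; When OnDisplay is false, Tick clears that player's heavy-item flag.
; Hitting anything but a player character stops projectile movement, enables physics and plays a drop sound.
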(event `self.ReceiveTick`
  (params (DeltaSeconds :type "Float (single-precision)"))
  (bind _player (`self.Player`))
  (bind _mesh (`self.Mesh`))
  (bind _mesh_2 (`self.Mesh`))
  (if (!= _player null)
    (if (`self.OnDisplay`)
      (`PrimitiveComponent.SetSimulatePhysics` _mesh_2 false)
      (`ActorComponent.Deactivate` (`self.ProjectileMovement`))
      (set `self.IsInAir` false)
      (`self.K2_AttachToComponent` (`Character.Mesh` _player) "Base-HumanPalmBone001Bone0015" "SnapToTarget" "SnapToTarget" "KeepWorld")
      (`PrimitiveComponent.SetCollisionProfileName` _mesh_2 "Trigger" true)
      (if (not (`self.cacheGrabbed`))
        (`SceneComponent.K2_AddLocalOffset` _mesh (20.0 -5.0 -4.934058) false false)
        (`SceneComponent.K2_AddLocalRotation` _mesh (struct :`Pitch` 50.0 :`Yaw` 10.0 :`Roll` 10.0) false false)
        (set `self.cacheGrabbed` true))
      (else
        (set `PlayerCharacter.IsHoldingHeavyItem` false _player)))
    (else
      (set `self.cacheGrabbed` false))))

(event `self.ReceiveHit`
  (params (MyComp :type "PrimitiveComponent Object Reference") (Other :type "Actor Object Reference") (OtherComp :type "PrimitiveComponent Object Reference") (bSelfMoved :type Boolean) (HitLocation :type "Vector Structure") (HitNormal :type "Vector Structure") (NormalImpulse :type "Vector Structure") (Hit :type "HitResult Structure (by ref)"))
  (cast `/Game/OneStarPrison/Blueprints/BP_PlayerCharacter` Other
    (:`CastFailed`
      (`PrimitiveComponent.SetSimulatePhysics` (`self.Mesh`) true)
      (`ActorComponent.Deactivate` (`self.ProjectileMovement`))
      (set `self.IsInAir` false)
      (`GameplayStatics.PlaySoundAtLocation` "/Game/OneStarPrison/Sounds/BarreDrop.BarreDrop" (`self.K2_GetActorLocation`) (struct) 1.0 1.0 0.0 "/Game/OneStarPrison/Sounds/AttentuationSettings/RockAttenuation.RockAttenuation" null null null))))

(fn `UserConstructionScript`)