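; Single-use pickupable small rock that makes one noise on impact as a projectile and is then destroyed.
; Hitting anything but the player switches it from projectile movement to physics, plays a rock sound and reports a noise event once for AI hearing.
; Once that noise flag is set, Tick clears the player's picked-up item reference and destroys the actor after a short delay.
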(event `self.ReceiveHit`
  (params (MyComp :type "PrimitiveComponent Object Reference") (Other :type "Actor Object Reference") (OtherComp :type "PrimitiveComponent Object Reference") (bSelfMoved :type Boolean) (HitLocation :type "Vector Structure") (HitNormal :type "Vector Structure") (NormalImpulse :type "Vector Structure") (Hit :type "HitResult Structure (by ref)"))
  (bind _returnvalue (`self.K2_GetActorLocation`))
  (cast `/Game/OneStarPrison/Blueprints/BP_PlayerCharacter` Other
    (:`CastFailed`
      (`PrimitiveComponent.SetSimulatePhysics` (`self.Mesh`) true)
      (`ActorComponent.Deactivate` (`self.ProjectileMovement`))
      (set `self.IsInAir` false)
      (`GameplayStatics.PlaySoundAtLocation` "/Game/OneStarPrison/Sounds/rock1.rock1" _returnvalue (struct) 1.0 1.0 0.0 "/Game/OneStarPrison/Sounds/AttentuationSettings/RockAttenuation.RockAttenuation" null null null)
      (if (not (`self.playedNoise`))
        (`AISense_Hearing.ReportNoiseEvent` _returnvalue 1.0 self)
        (set `self.playedNoise` true)))))

(event `self.ReceiveTick`
  (params (DeltaSeconds :type "Float (single-precision)"))
  (bind _player (`self.Player`))
  (if (`self.playedNoise`)
    (if (!= _player null)
      (set `PlayerCharacter.PickedUpItem` null _player))
    (`KismetSystemLibrary.Delay` 1.0)
    (`self.K2_DestroyActor`)))

(fn `UserConstructionScript`)