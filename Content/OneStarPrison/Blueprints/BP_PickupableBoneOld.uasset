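; Pickupable bone that players can carry and throw, making a noise on impact.
; Hitting anything but a player switches it from projectile movement to physics, plays a rock sound and reports a "Bone" noise event, only once per bone.
; Tick polls attachment to a player to track pickup and holding, destroying a released bone five seconds after impact.
; Damage reduces health, and a hit exceeding what remains destroys it.
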(event `self.ReceiveHit`
  (params (MyComp :type "PrimitiveComponent Object Reference") (Other :type "Actor Object Reference") (OtherComp :type "PrimitiveComponent Object Reference") (bSelfMoved :type Boolean) (HitLocation :type "Vector Structure") (HitNormal :type "Vector Structure") (NormalImpulse :type "Vector Structure") (Hit :type "HitResult Structure (by ref)"))
  (bind _returnvalue (`self.K2_GetActorLocation`))
  (cast `/Game/OneStarPrison/Blueprints/BP_PlayerCharacter` Other
    (:`CastFailed`
      (`PrimitiveComponent.SetSimulatePhysics` (`self.Mesh`) true)
      (`ActorComponent.Deactivate` (`self.ProjectileMovement`))
      (set `self.IsInAir` false)
      (`GameplayStatics.PlaySoundAtLocation` "/Game/OneStarPrison/Sounds/rock0.rock0" _returnvalue (struct) 1.0 1.0 0.0 "/Game/OneStarPrison/Sounds/AttentuationSettings/RockAttenuation.RockAttenuation" null null null)
      (set `self.Hitted ground` true)
      (if (not (`self.playedNoise`))
        (`AISense_Hearing.ReportNoiseEvent` _returnvalue 1.0 self 0.0 "Bone")
        (set `self.playedNoise` true)))))

(event `self.ReceiveTick`
  (params (DeltaSeconds :type "Float (single-precision)"))
  (`self.CheckPickedUp`)
  (`self.CheckPlayerHolding`)
  (if (`self.PickedUp`)
    (if (`self.Holding`)
      _
      (elif (`self.Hitted ground`)
        (set `self.TimePast` (+ DeltaSeconds (`self.TimePast`)))
        (if (>= (`self.TimePast`) 5.0)
          (`self.K2_DestroyActor`))))))

(event `self.ReceiveAnyDamage`
  (params (Damage :type "Float (single-precision)") (DamageType :type "DamageType Object Reference") (InstigatedBy :type "Controller Object Reference") (DamageCauser :type "Actor Object Reference"))
  (bind _health (`self.Health`))
  (if (> Damage _health)
    (`self.Destory_Mul`)
    (else
      (set `self.Health` (- _health Damage)))))

(event `Destory_Mul`
  (`self.K2_DestroyActor`))

(fn `CheckPickedUp`
  (bind _returnvalue (`self.GetAttachParentActor` self))
  (if (`self.PickedUp`)
    _
    (elif (!= _returnvalue null)
      (cast `/Game/OneStarPrison/Blueprints/BP_PlayerCharacter` _returnvalue)
      (set `self.PickedUp` true))))

(fn `CheckPlayerHolding`
  (bind _returnvalue (`self.GetAttachParentActor` self))
  (if (!= _returnvalue null)
    (cast `/Game/OneStarPrison/Blueprints/BP_PlayerCharacter` _returnvalue)
    (set `self.Holding` true)
    (set `self.Hitted ground` false)
    (set `self.TimePast` 0.0)
    (else
      (set `self.Holding` false))))

(fn `UserConstructionScript`)