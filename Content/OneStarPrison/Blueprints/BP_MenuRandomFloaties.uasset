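; Menu floatie actor that shows a random mesh drifting and spinning, judging by its name as decoration for the menu.
; On BeginPlay, Randomise picks a mesh from RandomFloaties (its Length minus one bound excludes the last entry) and prints the result, then the start location is stored but never read here.
; Each Tick moves the mesh by DifferentSpeed in world space and rotates it locally by DifferentRotation, without delta-time scaling.
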(event `self.ReceiveBeginPlay`
  (`self.Randomise`)
  (set `self.StartLocation` (`self.K2_GetActorLocation`)))

(event `self.ReceiveTick`
  (params (DeltaSeconds :type "Float (single-precision)"))
  (`SceneComponent.K2_AddWorldOffset` (`self.StaticMesh`) (`self.Different Speed`) false false)
  (`SceneComponent.K2_AddLocalRotation` (`self.StaticMesh`) (`self.Different Rotation`) false false))

(fn `Randomise`
  (bind _randomfloaties (`self.RandomFloaties`))
  (bind _returnvalue (`StaticMeshComponent.SetStaticMesh` (`self.StaticMesh`) (`|GetArrayItem` _randomfloaties (`KismetMathLibrary.RandomInteger` (- (`KismetArrayLibrary.Array_Length` _randomfloaties) 1)))))
  (`KismetSystemLibrary.PrintString` (`KismetStringLibrary.Conv_BoolToString` _returnvalue)))

(fn `UserConstructionScript`)