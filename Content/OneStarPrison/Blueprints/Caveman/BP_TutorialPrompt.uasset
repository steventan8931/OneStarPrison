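; BP_TutorialPrompt is an actor that pauses the game when the player character overlaps it, apparently as a tutorial beat.
; The overlap sets a Collided flag, which gates a Tick path that runs a one-second Delay, prints Timer plus delta seconds, then unpauses.
; Collided is never reset and Timer is never written here, and no prompt display is implemented.
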(event `self.ReceiveActorBeginOverlap`
  (params (OtherActor :type "Actor Object Reference"))
  (cast `/Game/OneStarPrison/Blueprints/BP_PlayerCharacter` OtherActor)
  (set `self.Collided` true)
  (`GameplayStatics.SetGamePaused` true))

(event `self.ReceiveTick`
  (params (DeltaSeconds :type "Float (single-precision)"))
  (if (`self.Collided`)
    (`KismetSystemLibrary.Delay` 1.0)
    (`KismetSystemLibrary.PrintString` (`KismetStringLibrary.Conv_DoubleToString` (+ (`self.Timer`) DeltaSeconds)))
    (`GameplayStatics.SetGamePaused` false)))

(fn `UserConstructionScript`)