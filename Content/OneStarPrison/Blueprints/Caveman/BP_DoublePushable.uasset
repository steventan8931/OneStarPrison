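; Pushable cooperative object that is meant to move only when two players push it together.
; A Box overlap tracks player characters and toggles their CanPush, while hitting the Mesh sets IsPushing.
; With exactly two players inside, Tick accumulates NumPlayersPushing, resets it after a Delay for non-pushers, and enables Mesh physics once it reaches two.
; Any other player count switches physics off and clears the counter.
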(event `self.ReceiveTick`
  (params (DeltaSeconds :type "Float (single-precision)"))
  (bind _mesh (`self.Mesh`))
  (if (== (`KismetArrayLibrary.Array_Length` (`self.Players`)) 2)
    (for _array_element (`self.Players`)
      (if (`PlayerCharacter.IsPushing` _array_element)
        (`/Engine/EditorBlueprintResources/StandardMacros.IncrementInt` (`self.NumPlayersPushing`))
        (else
          (`KismetSystemLibrary.Delay` 1.0)
          (set `self.NumPlayersPushing` 0))))
    (if (>= (`self.NumPlayersPushing`) 2)
      (`PrimitiveComponent.SetSimulatePhysics` _mesh true))
    (else
      (`PrimitiveComponent.SetSimulatePhysics` _mesh false)
      (set `self.NumPlayersPushing` 0))))

(event `self.Box.OnComponentBeginOverlap`
  (params (OverlappedComponent :type "PrimitiveComponent Object Reference") (OtherActor :type "Actor Object Reference") (OtherComp :type "PrimitiveComponent Object Reference") (OtherBodyIndex :type Integer) (bFromSweep :type Boolean) (SweepResult :type "HitResult Structure (by ref)"))
  (bind _asbp_player_character (cast `/Game/OneStarPrison/Blueprints/BP_PlayerCharacter` OtherActor))
  (set `PlayerCharacter.CanPush` true _asbp_player_character)
  (`KismetArrayLibrary.Array_Add` (`self.Players`) _asbp_player_character))

(event `self.Box.OnComponentEndOverlap`
  (params (OverlappedComponent :type "PrimitiveComponent Object Reference") (OtherActor :type "Actor Object Reference") (OtherComp :type "PrimitiveComponent Object Reference") (OtherBodyIndex :type Integer))
  (bind _asbp_player_character (cast `/Game/OneStarPrison/Blueprints/BP_PlayerCharacter` OtherActor))
  (set `PlayerCharacter.CanPush` false _asbp_player_character)
  (set `PlayerCharacter.IsPushing` false _asbp_player_character)
  (`KismetArrayLibrary.Array_RemoveItem` (`self.Players`) _asbp_player_character))

(event `self.Mesh.OnComponentHit`
  (params (HitComponent :type "PrimitiveComponent Object Reference") (OtherActor :type "Actor Object Reference") (OtherComp :type "PrimitiveComponent Object Reference") (NormalImpulse :type "Vector Structure") (Hit :type "HitResult Structure (by ref)"))
  (bind _asbp_player_character (cast `/Game/OneStarPrison/Blueprints/BP_PlayerCharacter` OtherActor))
  (set `PlayerCharacter.IsPushing` true _asbp_player_character))

(fn `UserConstructionScript`)