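; BP_DeathRock is a rock hazard that kills the player on contact.
; Both the actor Hit event and the Mesh component hit event cast the other actor to BP_PlayerCharacter and set its IsDead flag.
; Tick sets the Audio component's volume multiplier to half once DeathTime reaches a three-second threshold, though nothing in these graphs updates DeathTime.
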(event `self.ReceiveTick`
  (params (DeltaSeconds :type "Float (single-precision)"))
  (if (>= (`self.DeathTime`) 3.0)
    (`AudioComponent.SetVolumeMultiplier` (`self.Audio`) 0.5)))

(event `self.ReceiveHit`
  (params (MyComp :type "PrimitiveComponent Object Reference") (Other :type "Actor Object Reference") (OtherComp :type "PrimitiveComponent Object Reference") (bSelfMoved :type Boolean) (HitLocation :type "Vector Structure") (HitNormal :type "Vector Structure") (NormalImpulse :type "Vector Structure") (Hit :type "HitResult Structure (by ref)"))
  (bind _asbp_player_character (cast `/Game/OneStarPrison/Blueprints/BP_PlayerCharacter` Other))
  (set `PlayerCharacter.IsDead` true _asbp_player_character))

(event `self.Mesh.OnComponentHit`
  (params (HitComponent :type "PrimitiveComponent Object Reference") (OtherActor :type "Actor Object Reference") (OtherComp :type "PrimitiveComponent Object Reference") (NormalImpulse :type "Vector Structure") (Hit :type "HitResult Structure (by ref)"))
  (bind _asbp_player_character (cast `/Game/OneStarPrison/Blueprints/BP_PlayerCharacter` OtherActor))
  (set `PlayerCharacter.IsDead` true _asbp_player_character))

(fn `UserConstructionScript`)