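; Lobby portal trigger for one era (Caveman, Medieval or Pirate) that sends players into that era's level.
; On BeginPlay it reads the save slot to set unlock, free-play and Niagara visibility, with Caveman always unlocked.
; Overlapping players get era-specific model options and the character select UI, and leaving clears their ready state.
; Tick waits for two players, all ready, then server-travels to MapName and removes the UI.
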(event `SetModelOptions`
  (params (Player :type "/Game/OneStarPrison/Blueprints/BP_PlayerCharacter Object Reference"))
  (switch `/Game/OneStarPrison/Enumerations/ELevelEras` (`self.Era`)
    (:`NewEnumerator0`
      (set `/Game/OneStarPrison/Blueprints/BP_PlayerCharacter.ModelOptionF` "NewEnumerator5" Player)
      (set `/Game/OneStarPrison/Blueprints/BP_PlayerCharacter.ModelOptionM` "NewEnumerator2" Player))
    (:`NewEnumerator1`
      (set `/Game/OneStarPrison/Blueprints/BP_PlayerCharacter.ModelOptionF` "NewEnumerator1" Player)
      (set `/Game/OneStarPrison/Blueprints/BP_PlayerCharacter.ModelOptionM` "NewEnumerator0" Player))
    (:`NewEnumerator2`
      (set `/Game/OneStarPrison/Blueprints/BP_PlayerCharacter.ModelOptionF` "NewEnumerator4" Player)
      (set `/Game/OneStarPrison/Blueprints/BP_PlayerCharacter.ModelOptionM` "NewEnumerator3" Player))))

(event `Load Game`
  (bind _niagara (`self.Niagara`))
  (bind _returnvalue (`GameplayStatics.LoadGameFromSlot` "1"))
  (if (!= _returnvalue null)
    (bind _asbp_level_completion_save (cast `/Game/OneStarPrison/Saves/BP_LevelCompletionSave` _returnvalue)
      (:`then`
        (switch `/Game/OneStarPrison/Enumerations/ELevelEras` (`self.Era`)
          (:`NewEnumerator0`
            (bind _output_get (set `self.Unlocked` true))
            (bind _output_get_2 (set `self.Completed` (`.Completed_3_86BF56D14EA10AE7B4A20BA9CAF624C4` (break `/Game/OneStarPrison/Saves/F_LevelStatus` (`/Game/OneStarPrison/Saves/BP_LevelCompletionSave.Caveman` _asbp_level_completion_save)))))
            (`SceneComponent.SetVisibility` _niagara _output_get false)
            (set `self.IsFreePlay` _output_get_2))
          (:`NewEnumerator1`
            (bind (_unlocked _completed) (break `/Game/OneStarPrison/Saves/F_LevelStatus` (`/Game/OneStarPrison/Saves/BP_LevelCompletionSave.Medieval` _asbp_level_completion_save)))
            (bind _output_get_3 (set `self.Unlocked` _unlocked))
            (bind _output_get_4 (set `self.Completed` _completed))
            (`SceneComponent.SetVisibility` _niagara _output_get_3 false)
            (set `self.IsFreePlay` _output_get_4))
          (:`NewEnumerator2`
            (bind (_unlocked_2 _completed_2) (break `/Game/OneStarPrison/Saves/F_LevelStatus` (`/Game/OneStarPrison/Saves/BP_LevelCompletionSave.Pirate` _asbp_level_completion_save)))
            (bind _output_get_5 (set `self.Unlocked` _unlocked_2))
            (bind _output_get_6 (set `self.Completed` _completed_2))
            (`SceneComponent.SetVisibility` _niagara _output_get_5 false)
            (set `self.IsFreePlay` _output_get_6))))
      (:`CastFailed`
        (switch `/Game/OneStarPrison/Enumerations/ELevelEras` (`self.Era`) :!label _label
          (:`NewEnumerator0`
            (set `self.Unlocked` true)
            (set `self.Completed` false)
            (set `self.IsFreePlay` false))
          (:`NewEnumerator1`
            ;[1 1 1] set false for actual
            (bind _output_get_7 (set `self.Unlocked` false :!label _label_2))
            (set `self.Completed` false)
            (set `self.IsFreePlay` false)
            (`SceneComponent.SetVisibility` _niagara _output_get_7 false))
          (:`NewEnumerator2`
            (goto _label_2)))))
    (else
      (goto _label))))

(event `self.ReceiveBeginPlay`
  (`self.Load Game `))

(event `self.ReceiveActorBeginOverlap`
  (params (OtherActor :type "Actor Object Reference"))
  (if (`self.Unlocked`)
    (bind _asbp_player_character (cast `/Game/OneStarPrison/Blueprints/BP_PlayerCharacter` OtherActor))
    (set `self.PlayerCount` (+ (`self.PlayerCount`) 1))
    (`self.SetModelOptions` _asbp_player_character)
    (`/Game/OneStarPrison/Blueprints/BP_PlayerCharacter.ServerCharacterSelect` _asbp_player_character (`self.IsFreePlay`))
    (`KismetArrayLibrary.Array_Add` (`self.Players`) _asbp_player_character)))

(event `self.ReceiveActorEndOverlap`
  (params (OtherActor :type "Actor Object Reference"))
  (if (`self.Unlocked`)
    (bind _asbp_player_character (cast `/Game/OneStarPrison/Blueprints/BP_PlayerCharacter` OtherActor))
    (set `self.PlayerCount` (+ (`self.PlayerCount`) -1))
    (`/Game/OneStarPrison/Blueprints/BP_PlayerCharacter.ServerRemoveCharacterSelect` _asbp_player_character (`self.IsFreePlay`))
    (set `/Game/OneStarPrison/Blueprints/BP_PlayerCharacter.IsReady` false _asbp_player_character)
    (`KismetArrayLibrary.Array_RemoveItem` (`self.Players`) _asbp_player_character)))

(event `self.ReceiveTick`
  (params (DeltaSeconds :type "Float (single-precision)"))
  (if (== (`self.PlayerCount`) 2)
    (`self.CheckIsReady`)
    (if (`self.LobbyReady`)
      (`self.Change Level`)
      (`self.RemoveUI`))))

(event `Change Level`
  (`KismetSystemLibrary.ExecuteConsoleCommand` (`KismetStringLibrary.Concat_StrStr` "servertravel " (`self.MapName`)) (`GameplayStatics.GetPlayerController` 0))
  (`WidgetLayoutLibrary.RemoveAllWidgets`))

(fn `CheckIsReady`
  (for _array_element (`self.Players`)
    (if (`/Game/OneStarPrison/Blueprints/BP_PlayerCharacter.IsReady` _array_element)
      (set `self.LobbyReady` true)
      (else
        (set `self.LobbyReady` false)
        (break)))))

(fn `RemoveUI`
  (for _array_element (`self.Players`)
    (`/Game/OneStarPrison/Blueprints/BP_PlayerCharacter.ServerRemoveCharacterSelect` _array_element false)))

(fn `UserConstructionScript`)