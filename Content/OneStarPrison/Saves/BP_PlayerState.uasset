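; BP_PlayerState is a player state that stores the chosen character model and applies it to the player character.
; UpdateModel casts player 0's pawn to BP_PlayerCharacter, sets its ModelType, and switches on SavedModel to call UpdateCharacterModel for one of six themed male or female models.
; CopyProperties passes SavedModel to the new player state, so the selection survives player state replacement.
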(event `Update Model`
  (bind _saved_model (`self.Saved Model`))
  (bind _asbp_player_character (cast `/Game/OneStarPrison/Blueprints/BP_PlayerCharacter` (`GameplayStatics.GetPlayerCharacter` 0)))
  (set `/Game/OneStarPrison/Blueprints/BP_PlayerCharacter.ModelType` _saved_model _asbp_player_character)
  (switch `/Game/OneStarPrison/Enumerations/ECharacterModel` _saved_model
    (:`NewEnumerator0`
      (`/Game/OneStarPrison/Blueprints/BP_PlayerCharacter.Update Character Model` _asbp_player_character "NewEnumerator0"))
    (:`NewEnumerator1`
      (`/Game/OneStarPrison/Blueprints/BP_PlayerCharacter.Update Character Model` _asbp_player_character "NewEnumerator1"))
    (:`NewEnumerator2`
      (`/Game/OneStarPrison/Blueprints/BP_PlayerCharacter.Update Character Model` _asbp_player_character "NewEnumerator2"))
    (:`NewEnumerator5`
      (`/Game/OneStarPrison/Blueprints/BP_PlayerCharacter.Update Character Model` _asbp_player_character "NewEnumerator5"))
    (:`NewEnumerator3`
      (`/Game/OneStarPrison/Blueprints/BP_PlayerCharacter.Update Character Model` _asbp_player_character "NewEnumerator3"))
    (:`NewEnumerator4`
      (`/Game/OneStarPrison/Blueprints/BP_PlayerCharacter.Update Character Model` _asbp_player_character "NewEnumerator4"))))

(event `self.ReceiveBeginPlay`)

(event `self.ReceiveCopyProperties`
  (params (NewPlayerState :type "PlayerState Object Reference"))
  (bind _asbp_player_state (cast `/Game/OneStarPrison/Saves/BP_PlayerState` NewPlayerState))
  (set `/Game/OneStarPrison/Saves/BP_PlayerState.Saved Model` (`self.Saved Model`) _asbp_player_state))

(event `self.ReceiveDestroyed`)

(fn `UserConstructionScript`)