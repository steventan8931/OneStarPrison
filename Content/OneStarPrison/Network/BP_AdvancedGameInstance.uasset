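; Game instance for One Star Prison that handles multiplayer sessions and applies the saved character model to the player.
; Host destroys any existing session, then creates an advanced session tagged with a game name; Join finds a friend's session, and accepted invites join directly.
; UpdateModel maps the saved model type to one of six character models on player zero.
; Init deletes save slot "1", a development reset marked for removal to keep level completion.
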(event `Update Model`
  (bind _asbp_player_character (cast `/Game/OneStarPrison/Blueprints/BP_PlayerCharacter` (`GameplayStatics.GetPlayerCharacter` 0)))
  (switch `/Game/OneStarPrison/Enumerations/ECharacterModel` (`self.Saved Model Type`)
    (:`NewEnumerator0`
      (`/Game/OneStarPrison/Blueprints/BP_PlayerCharacter.Update Character Model` _asbp_player_character "NewEnumerator0"))
    (:`NewEnumerator1`
      (`/Game/OneStarPrison/Blueprints/BP_PlayerCharacter.Update Character Model` _asbp_player_character "NewEnumerator1"))
    (:`NewEnumerator2`
      (`/Game/OneStarPrison/Blueprints/BP_PlayerCharacter.Update Character Model` _asbp_player_character "NewEnumerator2"))
    (:`NewEnumerator5`
      (`/Game/OneStarPrison/Blueprints/BP_PlayerCharacter.Update Character Model` _asbp_player_character "NewEnumerator5"))
    (:`NewEnumerator3`
      (`/Game/OneStarPrison/Blueprints/BP_PlayerCharacter.Update Character Model` _asbp_player_character "NewEnumerator3"))
    (:`NewEnumerator4`
      (`/Game/OneStarPrison/Blueprints/BP_PlayerCharacter.Update Character Model` _asbp_player_character "NewEnumerator4"))))

(event `Join`
  (params (PlayerController :type "PlayerController Object Reference") (FriendUniqueNetId :type "BPUniqueNetId Structure (by ref)"))
  (bind _sessioninfo (`FindFriendSessionCallbackProxy.FindFriendSession` PlayerController FriendUniqueNetId)
    (:`OnSuccess`
      (`JoinSessionCallbackProxy.JoinSession` PlayerController (`|GetArrayItem` _sessioninfo)
        (:`OnSuccess`
          (`KismetSystemLibrary.PrintString` "Session Found"))
        (:`OnFailure`
          (`KismetSystemLibrary.PrintString` "Cant Join Session"))))))

(event `Host`
  (params (PlayerController :type "PlayerController Object Reference") (GameName :type String))
  ;[1 1 1] Added
  (`DestroySessionCallbackProxy.DestroySession` PlayerController
    (:`OnSuccess`
      _)
    (:`OnFailure`
      _))
  (`CreateSessionCallbackProxyAdvanced.CreateAdvancedSession` (`|MakeArray` (`AdvancedSessionsLibrary.MakeLiteralSessionPropertyString` "GameName" GameName)) PlayerController
    (:`OnSuccess`
      (`KismetSystemLibrary.PrintString` "Host Success"))
    (:`OnFailure`
      (`KismetSystemLibrary.PrintString` "No Session"))))

(event `self.ReceiveInit`
  ;[1 1 1] Remove to DELETE IN BUILD to keep level completion through sessions
  (`GameplayStatics.DeleteGameInSlot` "1"))

(event `self.OnSessionInviteAccepted`
  (params (LocalPlayerNum :type Integer) (PersonInvited :type "BPUniqueNetId Structure") (SessionToJoin :type "BlueprintSessionResult Structure (by ref)"))
  (`JoinSessionCallbackProxy.JoinSession` (`GameplayStatics.GetPlayerController` 0) SessionToJoin))